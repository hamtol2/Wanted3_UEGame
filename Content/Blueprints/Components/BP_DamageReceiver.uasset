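; BP_DamageReceiver is a component that tracks health and applies incoming damage.
; It fills HealthPower to MaxHealthPower on BeginPlay, then subtracts damage each time OnDamageReceived fires.
; At zero or below it clamps health to zero and broadcasts OnDead.
; Every hit also broadcasts OnHealthPowerChanged with current and max health, including the fatal one.
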(event Custom|OnDamageReceived
  (params (Damage :type Float%20%28double-precision%29))
  ;[0.15 0.15 0.15 0.5] 대미지 처리 공식
  (Variables|Default|SetHealthPower (- (Variables|Default|GetHealthPower) Damage))
  (if (<= (Variables|Default|GetHealthPower) 0.0)
    (Variables|Default|SetHealthPower 0.0)
    (Default|CallOnDead)
    (Default|CallOnHealthPowerChanged (Variables|Default|GetHealthPower) (Variables|Default|GetMaxHealthPower))
    (else
      (Default|CallOnHealthPowerChanged (Variables|Default|GetHealthPower) (Variables|Default|GetMaxHealthPower)))))

(event EventBeginPlay
  ;[0.15 0.15 0.15 0.5] 시작할 때 체력 채우기
  (Variables|Default|SetHealthPower (Variables|Default|GetMaxHealthPower)))